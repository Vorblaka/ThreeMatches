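; BP_SlowBombTower is a tower that damages and slows the enemy returned by GetClosestEnemy.
; DealDamage places a damage decal at the target, then hits either all overlapped pawns or only the target, depending on DamageRadius.
; Each BP_EnemyBase hit has its current MaxWalkSpeed scaled down, so repeated hits compound and nothing here restores the speed.
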(event EventDealDamage
  (bind _enemy (CallFunction|GetClosestEnemy))
  (Utilities|IsValid _enemy
    (:Is%20Valid
      (CallFunction|DamageDecal (Transformation|GetActorLocation _enemy))
      (if (> (Variables|Default|GetDamageRadius) 1.0)
        (bind _outactors (Collision|SphereOverlapActors (Transformation|GetActorLocation (.Enemy (CallFunction|GetClosestEnemy))) (Variables|Default|GetDamageRadius) (Utilities|Array|MakeArray "ObjectTypeQuery3") 0))
        (for _array_element _outactors
          (Game|Damage|ApplyDamage _array_element (Variables|Default|GetDamage) 0 self)
          (bind _asbp_enemy_base (Utilities|Casting|CastToBP_EnemyBase _array_element))
          (Variables|/Script/Engine.CharacterMovementComponent|SetMaxWalkSpeed (Variables|/Script/Engine.Character|GetCharacterMovement _asbp_enemy_base) (* (Variables|/Script/Engine.CharacterMovementComponent|GetMaxWalkSpeed (Variables|/Script/Engine.Character|GetCharacterMovement _asbp_enemy_base)) 0.7)))
        (else
          (Game|Damage|ApplyDamage _enemy (Variables|Default|GetDamage) 0 self)
          (bind _asbp_enemy_base_2 (Utilities|Casting|CastToBP_EnemyBase _enemy))
          (Variables|/Script/Engine.CharacterMovementComponent|SetMaxWalkSpeed (Variables|/Script/Engine.Character|GetCharacterMovement _asbp_enemy_base_2) (* (Variables|/Script/Engine.CharacterMovementComponent|GetMaxWalkSpeed (Variables|/Script/Engine.Character|GetCharacterMovement _asbp_enemy_base_2)) 0.7)))))))

(fn ConstructionScript
  (|CallParentFunction))