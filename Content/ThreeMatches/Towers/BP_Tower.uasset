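; BP_Tower is a tower that automatically fires on nearby enemies and expires shortly after its health component reports death.
; A range sphere, sized in construction along with the mesh collision, tracks overlapping BP_Enemy actors.
; After a growth delay, a looping timer spawns BP_Bullet at the closest valid enemy, pruning invalid entries.
; Bullet arrival triggers damage on whichever enemy is closest then, not necessarily the bullet's target.
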(event OnComponentBeginOverlap(AttackRangeCollision)
  (params (OverlappedComponent :type Primitive%20Component%20Object%20Reference) (OtherActor :type Actor%20Object%20Reference) (OtherComp :type Primitive%20Component%20Object%20Reference) (OtherBodyIndex :type Integer) (bFromSweep :type Boolean) (SweepResult :type Hit%20Result%20Structure%20%28by%20ref%29))
  (Class|KismetSystemLibrary|IsObjectOfSoftClass OtherActor "/Game/ThreeMatches/GIGI/BP_Enemy.BP_Enemy_C"
    (:True
      (Utilities|Array|Add (Variables|Default|GetEnemiesInRange) OtherActor))))

(event OnComponentEndOverlap(AttackRangeCollision)
  (params (OverlappedComponent :type Primitive%20Component%20Object%20Reference) (OtherActor :type Actor%20Object%20Reference) (OtherComp :type Primitive%20Component%20Object%20Reference) (OtherBodyIndex :type Integer))
  (Class|KismetSystemLibrary|IsObjectOfSoftClass OtherActor "/Game/ThreeMatches/GIGI/BP_Enemy.BP_Enemy_C"
    (:True
      (Utilities|Array|RemoveItem (Variables|Default|GetEnemiesInRange) OtherActor))))

(event OnDeath(ACO_Health)
  (Actor|SetLifeSpan 0.1))

(event Custom|Shoot
  (bind _enemy (CallFunction|GetClosestEnemy))
  (if (Utilities|Array|IsNotEmpty (Variables|Default|GetEnemiesInRange))
    (Utilities|IsValid _enemy
      (:Is%20Valid
        (bind _output_get (Variables|Default|SetBulletData (Utilities|Struct|MakeF_BulletData _enemy (.startingspeed (Variables|Default|GetBulletData)) (.acceleration (Variables|Default|GetBulletData)) (.maxspeed (Variables|Default|GetBulletData)) (.mesh (Variables|Default|GetBulletData)))))
        (bind _returnvalue (Game|SpawnActorfromClass "/Game/ThreeMatches/Towers/Bullets/BP_Bullet.BP_Bullet_C" (Transformation|GetActorTransform) "AdjustIfPossibleButAlwaysSpawn" "MultiplyWithRoot" 0 _output_get 0))
        (EventDispatchers|BindEventtoOnTargetReached _returnvalue (delegate Custom|DealDamage)))
      (:Is%20Not%20Valid
        (Utilities|Array|RemoveItem (Variables|Default|GetEnemiesInRange) _enemy)
        (CallFunction|Shoot)))))

(event Custom|DealDamage
  (Game|Damage|ApplyDamage (.Enemy (CallFunction|GetClosestEnemy)) (Variables|Default|GetDamage) 0 self))

(event EventBeginPlay
  (Utilities|Time|SetTimerbyEvent (delegate Custom|Shoot) (Variables|Default|GetFireInterval) true false (Variables|Default|GetGrowthDelay)))

(fn ConstructionScript
  (Components|Sphere|SetSphereRadius (Variables|Default|GetMeshCollision) (.sphereradius (StaticMesh|GetBounds (Variables|/Script/Engine.StaticMeshComponent|GetStaticMesh (Variables|Default|GetStaticMesh)))) true)
  (Components|Sphere|SetSphereRadius (Variables|Default|GetAttackRangeCollision) (Variables|Default|GetAttackRange) true))

(fn GetClosestEnemy
  (bind _output_get (LocalVariables|SetClosestEnemy (Utilities|Array|Get(acopy) (Variables|Default|GetEnemiesInRange))))
  (LocalVariables|SetPreviousDistance (Transformation|GetDistanceTo _output_get))
  (for _array_element (Variables|Default|GetEnemiesInRange)
    (if (> (LocalVariables|GetPreviousDistance) (Transformation|GetDistanceTo _array_element))
      (LocalVariables|SetPreviousDistance (Transformation|GetDistanceTo _array_element))
      (LocalVariables|SetClosestEnemy _array_element)))
  (return (LocalVariables|GetClosestEnemy) (LocalVariables|GetPreviousDistance)))