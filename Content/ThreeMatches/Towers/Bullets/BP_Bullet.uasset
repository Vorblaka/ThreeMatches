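; BP_Bullet is a homing tower projectile that flies toward its target actor, then fires OnTargetReached and destroys itself.
; A Data struct supplies the mesh, target and speed settings.
; Tick steps toward the target's current location without sweeping, detecting arrival using the mesh's bounding sphere radius as tolerance.
; Speed gains a fixed acceleration each frame, unscaled by delta time, up to a maximum; ShouldMove is set but never read here.
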(event Custom|TargetReached
  (Default|CallOnTargetReached)
  (Actor|DestroyActor))

(event EventTick
  (params (DeltaSeconds :type Float%20%28single-precision%29))
  (bind _data (Variables|Default|GetData))
  (Transformation|SetActorLocation (+ (* DeltaSeconds (Variables|Default|GetCurrentSpeed) (Math|Vector|GetUnitDirection(Vector) (Transformation|GetActorLocation) (Transformation|GetActorLocation (.target (Variables|Default|GetData))))) (Transformation|GetActorLocation)) false false)
  (if (Utilities|Operators|EqualEqual (Transformation|GetActorLocation) (Transformation|GetActorLocation (.target _data)) (.sphereradius (StaticMesh|GetBounds (.mesh _data))))
    (CallFunction|TargetReached)
    (else
      (Variables|Default|SetCurrentSpeed (Math|Float|Clamp(Float) (+ (Variables|Default|GetCurrentSpeed) (.acceleration _data)) (.startingspeed _data) (.maxspeed _data))))))

(event EventBeginPlay
  (bind _data (Variables|Default|GetData))
  (Variables|Default|SetCurrentSpeed (.startingspeed _data))
  (Components|StaticMesh|SetStaticMesh (Variables|Default|GetStaticMesh) (.mesh _data))
  (Variables|Default|SetShouldMove true))

(fn ConstructionScript)