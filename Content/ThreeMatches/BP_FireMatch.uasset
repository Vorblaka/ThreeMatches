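; Fire match effect in the ThreeMatches game that visualizes the castle core's remaining health as light.
; On BeginPlay it finds the arena and core, moves a scaled sphere proxy to the arena sphere, and places the Niagara fire relative to it.
; Each Tick, the scaled health ratio drives the proxy's dynamic material RemainingLight and the Niagara radius, and continually nudges the fire along Z.
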(event EventBeginPlay
  (bind _returnvalue (Actor|GetActorOfClass "/Game/ThreeMatches/GIGI/BP_Arena.BP_Arena_C"))
  (bind _output_get (Variables|Default|SetRealSphere _returnvalue))
  (bind _returnvalue_2 (Actor|GetActorOfClass "/Game/ThreeMatches/BP_CastleCore.BP_CastleCore_C"))
  (Variables|Default|SetCrystalCore _returnvalue_2)
  (Transformation|SetWorldTransform (Variables|Default|GetSphereProxy) (Math|Transform|MakeTransform (Transformation|GetWorldLocation (Variables|/Game/ThreeMatches/GIGI/BP_Arena.BP_Arena_C|GetSphere _output_get)) "0, 0, 0" "40.000000,40.000000,40.000000") false false)
  (Transformation|SetWorldLocation (Variables|Default|GetN_FireMatch) (* (Transformation|GetWorldLocation (Variables|/Game/ThreeMatches/GIGI/BP_Arena.BP_Arena_C|GetSphere _output_get)) (Variables|Default|GetRemainingLight)) false false))

(event EventTick
  (params (DeltaSeconds :type Float%20%28single-precision%29))
  (bind _crystalcore (Variables|Default|GetCrystalCore))
  (bind _n_firematch (Variables|Default|GetN_FireMatch))
  (bind _aco_health (Variables|/Game/ThreeMatches/BP_CastleCore.BP_CastleCore_C|GetACO_Health _crystalcore))
  (bind _current_health (Variables|/Game/ThreeMatches/Towers/ACO_Health.ACO_Health_C|GetCurrent%20Health _aco_health))
  (bind _maxhealth (Variables|/Game/ThreeMatches/Towers/ACO_Health.ACO_Health_C|GetMaxHealth _aco_health))
  (bind _returnvalue (* _maxhealth 5.0))
  (bind _returnvalue_2 (/ _current_health _returnvalue))
  (Rendering|Material|SetScalarParameterValue (Variables|Default|GetFireMatchMaterial) "RemainingLight" _returnvalue_2 :!class /Script/Engine.MaterialInstanceDynamic)
  (Niagara|SetNiagaraVariable(Float) _n_firematch "Radius" (* _returnvalue_2 1.5e+02))
  (Transformation|AddWorldOffset _n_firematch (Math|Vector|MakeVector 0.0 0.0 (* _returnvalue_2 1.0)) false false))

(fn ConstructionScript
  (Utilities|FlowControl|Sequence
    (:then_0
      (bind _returnvalue (Rendering|Material|CreateDynamicMaterialInstance (Variables|Default|GetSphereProxy) 0 "/Game/ThreeMatches/M_FireMatch_Inst.M_FireMatch_Inst" "None" :!class /Script/Engine.PrimitiveComponent))
      (Variables|Default|SetFireMatchMaterial _returnvalue)
      (Rendering|Material|SetScalarParameterValue (Variables|Default|GetFireMatchMaterial) "RemainingLight" (Variables|Default|GetRemainingLight) :!class /Script/Engine.MaterialInstanceDynamic))))