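; BP_Arena is the tower defence play surface where the selected tower gets placed.
; When selected, it asks BP_TowerDefencePlayerController whether that tower can spawn, then has the controller spawn it at the hit location and normal and plays a placement sound.
; If spawning is not allowed, it prints a message naming the tower and saying the player is too low on Hopes and Dreams.
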(event EventOnSelected
  (params (Instigator :type Object%20Object%20Reference) (Hit%20Result :type Hit%20Result%20Structure))
  (bind (_bblockinghit _binitialoverlap _time _distance _location _impactpoint _normal) (Collision|BreakHitResult Hit%20Result))
  (bind _asbp_tower_defence_player_controller (Utilities|Casting|CastToBP_TowerDefencePlayerController (Game|GetPlayerController 0)))
  (bind _can_spawn (Default|CanSpawnSelectedTower _asbp_tower_defence_player_controller))
  (if _can_spawn
    (Default|SpawnSelectedTower _asbp_tower_defence_player_controller _location _normal)
    (Audio|PlaySound2D "/Game/ThreeMatches/Sounds/Cue_PlaceTurret.Cue_PlaceTurret" 1.0 1.0 0.0 0 0)
    (else
      (Development|PrintText (Utilities|Text|FormatText "Cannot spawn '{Tower Name}', too low on Hopes and Dreams" (Default|GetSelectedTowerName (Variables|/Game/ThreeMatches/Systems/BP_TowerDefencePlayerController.BP_TowerDefencePlayerController_C|GetTower%20Placer _asbp_tower_defence_player_controller))) true true "(R=1.000000,G=0.200037,B=0.348831,A=1.000000)"))))

(fn ConstructionScript)