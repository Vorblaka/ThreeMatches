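; Base enemy pawn that heads for the torch and diverts to attack towers, with stats from an EnemyDefinition.
; A looping timer sphere-traces for a BP_Tower with health, falls back to the torch, and issues AIMoveTo.
; On arrival, a rate-limited attack re-traces and damages only a found tower, possibly not the current target.
; Health death broadcasts OnDead and destroys the actor; target-priority logic is unwired.
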(event OnDeath(ACO_Health)
  (CallFunction|Die))

(event Custom|Die
  (Default|CallOnDead self)
  (Actor|DestroyActor))

(event Custom|OnEnemyDecisionTick
  (bind _capsulecomponent (Variables|Collision|GetCapsuleComponent))
  (bind _returnvalue (Transformation|GetWorldLocation _capsulecomponent))
  (Utilities|FlowControl|Sequence
    (:then_0
      (bind _outhits (Collision|MultiSphereTraceByChannel _returnvalue _returnvalue (.EnemyPerceptionRadius (Utilities|Struct|BreakST_EnemyDefinition (Variables|Default|GetEnemyDefinition))) "TraceTypeQuery1" false 0 "None" true "(R=1.000000,G=0.000000,B=0.000000,A=1.000000)" "(R=0.000000,G=1.000000,B=0.000000,A=1.000000)" (Variables|Default|GetEnemyDecisionTickRate)))
      (bind (_targetactor _targethealthcomponent _bwassuccessful) (CallFunction|GetTargetfromSphereTrace _outhits))
      (if _bwassuccessful
        (Variables|Default|SetCurrentTarget _targetactor)
        (else
          (Variables|Default|SetCurrentTarget (Variables|Default|GetTorchTarget)))))
    (:then_1
      (AI|AIMoveTo self "0, 0, 0" (Variables|Default|GetCurrentTarget) (.EnemyAttackRange (Utilities|Struct|BreakST_EnemyDefinition (Variables|Default|GetEnemyDefinition))) true
        (:OnSuccess
          (Utilities|FlowControl|DoOnce false
            (:Completed
              (Utilities|Time|SetTimerbyEvent (delegate Custom|OnAttackReset) (.EnemyAttackRate (Utilities|Struct|BreakST_EnemyDefinition (Variables|Default|GetEnemyDefinition))))
              (CallFunction|Attack)
              (Variables|Default|SetbCanAttack false))))))))

(event Custom|InitializeEnemy
  (Variables|/Game/ThreeMatches/Towers/ACO_Health.ACO_Health_C|SetMaxHealth (Variables|Default|GetACO_Health) (.EnemyMaxHealth (Utilities|Struct|BreakST_EnemyDefinition (Variables|Default|GetEnemyDefinition))))
  (Utilities|Time|SetTimerbyEvent (delegate Custom|OnEnemyDecisionTick) (Variables|Default|GetEnemyDecisionTickRate) true true))

(event Custom|OnAttackReset
  (Variables|Default|SetbCanAttack true)
  (Utilities|FlowControl|DoOnce false) ; enters at Reset
)

(event EventTick
  (params (DeltaSeconds :type Float%20%28single-precision%29))
  (bind _currenttarget (Variables|Default|GetCurrentTarget))
  (if (Variables|Default|GetbShouldShowDebug)
    (Utilities|IsValid _currenttarget
      (:Is%20Valid
        (Rendering|Debug|DrawDebugLine (Transformation|GetWorldLocation (Variables|Collision|GetCapsuleComponent)) (Transformation|GetActorLocation _currenttarget) "(R=1.000000,G=0.017485,B=0.017166,A=1.000000)" (Variables|Default|GetEnemyDecisionTickRate) 1.0)))))

(event Game|Damage|EventAnyDamage
  (params (Damage :type Float%20%28single-precision%29) (DamageType :type Damage%20Type%20Object%20Reference) (InstigatedBy :type Controller%20Object%20Reference) (DamageCauser :type Actor%20Object%20Reference))
  (Audio|PlaySound2D "/Game/ThreeMatches/Sounds/Cue_EnemyHit.Cue_EnemyHit" 1.0 1.0 0.0 0 0))

(fn ConstructionScript)

(fn GetTargetfromSphereTrace
  (params (Array :type Array%20of%20Hit%20Result%20Structures))
  (bind _torchtarget (Variables|Default|GetTorchTarget))
  (bind _array_element (Utilities|Array|ForEachLoopwithBreak Array :!label _label)
    (:LoopBody
      (Utilities|Casting|CastToBP_Tower (.HitActor (Collision|BreakHitResult _array_element)))
      (LocalVariables|SetTargetComponentFound (Actor|GetComponentbyClass (.HitActor (Collision|BreakHitResult _array_element)) "/Game/ThreeMatches/Towers/ACO_Health.ACO_Health_C"))
      (goto _label Break))
    (:Completed
      (bind _targetcomponentfound (LocalVariables|GetTargetComponentFound)
        (:then
          (return (Components|GetOwner _targetcomponentfound) _targetcomponentfound true))
        (:else
          (return _torchtarget (Actor|GetComponentbyClass _torchtarget "/Game/ThreeMatches/Towers/ACO_Health.ACO_Health_C") false))))))

(fn Attack
  (bind _capsulecomponent (Variables|Collision|GetCapsuleComponent))
  (bind _returnvalue (Transformation|GetWorldLocation _capsulecomponent))
  (bind _outhits (Collision|MultiSphereTraceByChannel _returnvalue _returnvalue (+ (.EnemyAttackRange (Utilities|Struct|BreakST_EnemyDefinition (Variables|Default|GetEnemyDefinition))) 25.0) "TraceTypeQuery1" false 0 (CallFunction|ShouldShowSphereDebug) true "(R=1.000000,G=0.000000,B=0.000000,A=1.000000)" "(R=0.000000,G=1.000000,B=0.000000,A=1.000000)" (Variables|Default|GetEnemyDecisionTickRate)))
  ;[0.15 0.15 0.15 0.5] TODO This may attack a different object than the current target
  (bind (_targetactor _targethealthcomponent _bwassuccessful) (CallFunction|GetTargetfromSphereTrace _outhits))
  (if _bwassuccessful
    (Game|Damage|ApplyDamage _targetactor (.EnemyAttackDamage (Utilities|Struct|BreakST_EnemyDefinition (Variables|Default|GetEnemyDefinition))) 0 self)))

(fn ShouldShowSphereDebug
  (return (select (Variables|Default|GetbShouldShowDebug) "ForDuration" "None")))

(fn HasTowerPrioOverCastle
  (params (TowerPrio :type Float%20%28double-precision%29))
  (return (>= TowerPrio (.EnemyCastlePriority (Utilities|Struct|BreakST_EnemyDefinition (Variables|Default|GetEnemyDefinition))))))