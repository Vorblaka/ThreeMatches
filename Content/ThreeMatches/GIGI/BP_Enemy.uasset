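; BP_Enemy is an AI enemy that hunts towers on its way to a final target.
; InitializeEnemy sizes the perception sphere, constructs a work-in-progress BP_EnemyBehaviour and starts a looping decision timer.
; Each tick sphere-traces for a BP_Tower, falls back to FinalTarget, then uses AIMoveTo to approach within attack range, with debug drawing.
; Damage handling and RunEnemyBehaviour are empty stubs, and Die simply destroys the actor.
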(event Custom|Die
  (Actor|DestroyActor))

(event Custom|OnEnemyDecisionTick
  (bind _capsulecomponent (Variables|Collision|GetCapsuleComponent))
  (bind _returnvalue (Transformation|GetWorldLocation _capsulecomponent))
  (bind _outhits (Collision|MultiSphereTraceByChannel _returnvalue _returnvalue (Variables|Default|GetEnemyPerceptionRadius) "TraceTypeQuery1" false 0 "ForDuration" true "(R=1.000000,G=0.000000,B=0.000000,A=1.000000)" "(R=0.000000,G=1.000000,B=0.000000,A=1.000000)" (Variables|Default|GetEnemyDecisionTickRate)))
  (bind _target (CallFunction|GetTargetfromSphereTrace _outhits))
  (Variables|Default|SetCurrentTarget (select (Utilities|IsValid _target) _target (Variables|Default|GetFinalTarget)))
  (Rendering|Debug|DrawDebugLine (Transformation|GetWorldLocation (Variables|Collision|GetCapsuleComponent)) (Transformation|GetActorLocation (Variables|Default|GetCurrentTarget)) "(R=1.000000,G=0.017485,B=0.017166,A=1.000000)" (Variables|Default|GetEnemyDecisionTickRate) 1.0)
  (AI|AIMoveTo self "0, 0, 0" (Variables|Default|GetCurrentTarget) (Variables|Default|GetEnemyAttackRange) false))

(event Custom|InitializeEnemy
  (Components|Sphere|SetSphereRadius (Variables|Default|GetSphere) (Variables|Default|GetEnemyPerceptionRadius) true)
  ;[0.15 0.15 0.15 0.5] WIP
  (Game|ConstructObjectfromClass "/Game/ThreeMatches/GIGI/BP_EnemyBehaviour.BP_EnemyBehaviour_C" self (Variables|Default|GetFinalTarget))
  (Utilities|Time|SetTimerbyEvent (delegate Custom|OnEnemyDecisionTick) (Variables|Default|GetEnemyDecisionTickRate) true true))

(event Game|Damage|EventAnyDamage
  (params (Damage :type Float%20%28single-precision%29) (DamageType :type Damage%20Type%20Object%20Reference) (InstigatedBy :type Controller%20Object%20Reference) (DamageCauser :type Actor%20Object%20Reference)))

(fn ConstructionScript)

(fn RunEnemyBehaviour)

(fn GetTargetfromSphereTrace
  (params (Array :type Array%20of%20Hit%20Result%20Structures))
  (bind _array_element (Utilities|Array|ForEachLoopwithBreak Array :!label _label)
    (:LoopBody
      (bind _asbp_tower (Utilities|Casting|CastToBP_Tower (.HitActor (Collision|BreakHitResult _array_element))))
      (LocalVariables|SetTargetFound _asbp_tower)
      (goto _label Break))
    (:Completed
      (return (LocalVariables|GetTargetFound)))))