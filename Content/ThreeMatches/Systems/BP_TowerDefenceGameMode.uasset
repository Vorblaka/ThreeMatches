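; Tower defence game mode that runs a series of timed matches and records how long each one lasts.
; On BeginPlay it shows the mouse cursor, finds the encounter manager and binds to its encounter-end event and the player controller's start-play and main-menu events.
; Tick times the active match.
; Each encounter end stores that time, then triggers either the next play or game over; main menu clears the times.
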(event Custom|OnStartPlaying
  (Variables|Default|SetIsPlaying true))

(event Custom|EndMatch
  (Variables|Default|SetIsPlaying false)
  (Utilities|Array|Add (Variables|Default|GetMatchTimes) (Variables|Default|GetMatchTime))
  (Variables|Default|SetMatchTime 0.0)
  (bind _result (Math|Integer|DecrementInt (Variables|Default|GetMatchesNumber))
    (:%20%20
      (if (<= _result 0)
        (Default|GameOverMenu (Variables|Default|GetController))
        (Variables|Default|SetMatchesNumber (Variables|Default|GetMaxMatches))
        (else
          (Default|MenuPressPlay (Variables|Default|GetController) false))))))

(event Custom|OnMainMenu
  (Utilities|Array|Clear (Variables|Default|GetMatchTimes)))

(event EventBeginPlay
  (bind _returnvalue (Game|GetPlayerController 0))
  (Variables|/Script/Engine.PlayerController|SetbShowMouseCursor _returnvalue true)
  (Input|SetInputModeGameandUI _returnvalue 0 "DoNotLock" false false)
  (Variables|Default|SetMatchesNumber (Variables|Default|GetMaxMatches))
  (bind _returnvalue_2 (Actor|GetActorOfClass "/Game/ThreeMatches/GIGI/BP_EncounterManager.BP_EncounterManager_C"))
  (Utilities|IsValid _returnvalue_2
    (:Is%20Valid
      (bind _output_get (Variables|Default|SetEncounterManager _returnvalue_2))
      (EventDispatchers|BindEventtoOnEncounterEnd _output_get (delegate Custom|EndMatch))
      (bind _asbp_tower_defence_player_controller (Utilities|Casting|CastToBP_TowerDefencePlayerController (Game|GetPlayerController 0)))
      (bind _output_get_2 (Variables|Default|SetController _asbp_tower_defence_player_controller))
      (EventDispatchers|BindEventtoOnStartPlay _output_get_2 (delegate Custom|OnStartPlaying))
      (EventDispatchers|BindEventtoOnMainMenu _output_get_2 (delegate Custom|OnMainMenu)))))

(event EventTick
  (params (DeltaSeconds :type Float%20%28single-precision%29))
  (if (Variables|Default|GetIsPlaying)
    (Variables|Default|SetMatchTime (+ DeltaSeconds (Variables|Default|GetMatchTime)))))

(fn ConstructionScript)