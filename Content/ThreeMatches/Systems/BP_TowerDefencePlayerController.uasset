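; Player controller for the tower defence game, handling menu flow, input and the player's Hopes and Dreams resources.
; Menu, play and pause transitions swap widgets, input modes and Enhanced Input mapping contexts, while any key press detects gamepad switches.
; Clicks trace to I_ClickTarget actors, and rotation input tweens the pawn's spring arm in yaw steps.
; Tower spawning goes through TowerPlacer, aligns towers to the surface normal and deducts their Hopes cost.
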(event Custom|Start%20Game
  (params (FirstTime :type Boolean))
  (Default|CallOnStartGame FirstTime)
  (if FirstTime
    (Variables|Default|SetbShowMouseCursor true)
    (Variables|HopesandDreams|SetHopes (Variables|HopesandDreams|GetInitial%20Hopes))
    (Variables|HopesandDreams|SetDreams (Variables|HopesandDreams|GetInitial%20Dreams))))

(event Custom|EnterMenu
  (Viewport|RemoveAllWidgets)
  (bind _returnvalue (UserInterface|CreateWidget "/Game/ThreeMatches/UI/WBP_StartMenu.WBP_StartMenu_C" self))
  (Input|SetInputModeUIOnly self _returnvalue "DoNotLock" false)
  (UserInterface|Viewport|AddtoViewport _returnvalue 0)
  (CallFunction|SwapMappingContext true))

(event Custom|ResumeGame
  (Game|SetGamePaused false)
  (Viewport|RemoveAllWidgets)
  (bind _returnvalue (UserInterface|CreateWidget "/Game/ThreeMatches/UI/Widgets/WBP_TowerDefenceHUD.WBP_TowerDefenceHUD_C" self))
  (UserInterface|Viewport|AddtoViewport _returnvalue 0)
  (Input|SetInputModeGameOnly self false)
  (CallFunction|SwapMappingContext false))

(event Custom|MenuPressPlay
  (Default|CallOnMenuPressPlay)
  (Viewport|RemoveAllWidgets)
  (bind _returnvalue (UserInterface|CreateWidget "/Game/ThreeMatches/UI/Widgets/WBP_TowerDefenceHUD.WBP_TowerDefenceHUD_C" self))
  (UserInterface|Viewport|AddtoViewport _returnvalue 0)
  (Input|SetInputModeGameOnly self false)
  (CallFunction|SwapMappingContext false))

(event Input|EnhancedActionEvents|EnhancedInputActionIA_Click
  (params (ActionValue :type Boolean) (ElapsedSeconds :type Float%20%28double-precision%29) (TriggeredSeconds :type Float%20%28double-precision%29) (InputAction :type Input%20Action%20Object%20Reference :default "/Game/ThreeMatches/Systems/Input/TowerDefence/IA_Click.IA_Click"))
  (bind _array (Utilities|Array|MakeArray "ObjectTypeQuery1"))
  (bind (_hitresult _returnvalue) (Class|PlayerController|GetHitResultUnderCursorforObjects _array true))
  (bind _hitactor (Collision|BreakHitResult _hitresult))
  (if _returnvalue
    (if (Utilities|DoesObjectImplementInterface _hitactor "/Game/ThreeMatches/Interfaces/I_ClickTarget.I_ClickTarget_C")
      (Class|IClickTarget|OnSelected(Message) _hitactor self _hitresult))))

(event Input|EnhancedActionEvents|EnhancedInputActionIA_Pause
  (params (ActionValue :type Boolean) (ElapsedSeconds :type Float%20%28double-precision%29) (TriggeredSeconds :type Float%20%28double-precision%29) (InputAction :type Input%20Action%20Object%20Reference :default "/Game/ThreeMatches/Systems/Input/TowerDefence/IA_Pause.IA_Pause"))
  (Game|SetGamePaused true)
  (Viewport|RemoveAllWidgets)
  (bind _returnvalue (UserInterface|CreateWidget "/Game/ThreeMatches/UI/WBP_PauseMenu.WBP_PauseMenu_C" self))
  (Input|SetInputModeUIOnly self _returnvalue "DoNotLock" false)
  (UserInterface|Viewport|AddtoViewport _returnvalue 0)
  (CallFunction|SwapMappingContext true)
  (Variables|Default|SetbShowMouseCursor true))

(event Input|EnhancedActionEvents|EnhancedInputActionIA_Skip
  (params (ActionValue :type Boolean) (ElapsedSeconds :type Float%20%28double-precision%29) (TriggeredSeconds :type Float%20%28double-precision%29) (InputAction :type Input%20Action%20Object%20Reference :default "/Game/ThreeMatches/Systems/Input/TowerDefence/IA_Skip.IA_Skip"))
  (Default|CallRequestSkip))

(event Input|EnhancedActionEvents|EnhancedInputActionIA_Rotation
  (params (ActionValue :type Float%20%28double-precision%29) (ElapsedSeconds :type Float%20%28double-precision%29) (TriggeredSeconds :type Float%20%28double-precision%29) (InputAction :type Input%20Action%20Object%20Reference :default "/Game/ThreeMatches/Systems/Input/TowerDefence/IA_Rotation.IA_Rotation"))
  (Utilities|FlowControl|Sequence
    (:then_0
      (bind _alpha (Timeline|Rotation%20Tween Stop)
        (:Update
          (Transformation|SetRelativeRotation (Variables|Rotation|GetTarget%20Of%20Rotation) (Math|Rotator|Lerp(Rotator) (Variables|Rotation|GetRotation%20Start) (Variables|Rotation|GetRotation%20Destination) _alpha true) false false))))
    (:then_1
      (bind _asthree_matches_pawn_bp (Utilities|Casting|CastToThreeMatchesPawn_BP (Pawn|GetControlledPawn)))
      (Variables|Rotation|SetTarget%20Of%20Rotation (Variables|/Game/ThreeMatches/Systems/ThreeMatchesPawn_BP.ThreeMatchesPawn_BP_C|GetSpringArm _asthree_matches_pawn_bp))
      (bind _output_get (Variables|Rotation|SetRotation%20Start (Class|SpringArmComponent|GetTargetRotation (Variables|/Game/ThreeMatches/Systems/ThreeMatchesPawn_BP.ThreeMatchesPawn_BP_C|GetSpringArm _asthree_matches_pawn_bp))))
      (Variables|Rotation|SetRotation%20Destination (Math|Rotator|CombineRotators _output_get (Math|Rotator|MakeRotator 0.0 0.0 (* ActionValue 45.0 -1.0))))
      (Timeline|Rotation%20Tween PlayFromStart))))

(event Input|KeyboardEvents|AnyKey
  (params (Key :type Key%20Structure :default "None"))
  (:Pressed
    (if (!= (Class|KismetInputLibrary|KeyIsGamepadKey Key) (Variables|Input|GetIsUsingGamepad))
      (bind _output_get (Variables|Input|SetIsUsingGamepad (not (Variables|Input|GetIsUsingGamepad))))
      (Default|CallOnInputMethodChanged _output_get))))

(fn ConstructionScript)

(fn SpawnSelectedTower
  (params (Location :type Vector) (Normal :type Vector))
  (bind _spawned_tower (Default|SpawnSelectedTower (Variables|Default|GetTower%20Placer) (Math|Transform|MakeTransform Location (Math|Rotator|MakeRotfromZ Normal))))
  (Utilities|IsValid _spawned_tower
    (:Is%20Valid
      (Variables|HopesandDreams|SetHopes (- (Variables|HopesandDreams|GetHopes) (.hopescost (Default|GetSelectedTower (Variables|Default|GetTower%20Placer)))))
      (return _spawned_tower))))

(fn CanSpawnSelectedTower
  (return (not (< (- (Variables|HopesandDreams|GetHopes) (.hopescost (Default|GetSelectedTower (Variables|Default|GetTower%20Placer)))) 0.0))))

(fn AddHopes
  (params (Amount :type Float%20%28double-precision%29))
  (Variables|HopesandDreams|SetHopes (Math|Float|Clamp(Float) (+ Amount (Variables|HopesandDreams|GetHopes)) 0.0 (Variables|HopesandDreams|GetInitial%20Hopes))))

(fn AddDreams
  (params (Amount :type Float%20%28double-precision%29))
  (Variables|HopesandDreams|SetDreams (Math|Float|Clamp(Float) (+ Amount (Variables|HopesandDreams|GetDreams)) 0.0 (Variables|HopesandDreams|GetInitial%20Dreams))))

(fn SwapMappingContext
  (params (IsMenu :type Boolean))
  (bind _returnvalue (PlayerController|LocalPlayerSubsystems|GetEnhancedInputLocalPlayerSubsystem))
  (Utilities|IsValid _returnvalue
    (:Is%20Valid
      (if IsMenu
        (Input|RemoveMappingContext _returnvalue "/Game/ThreeMatches/Systems/Input/TowerDefence/IMC_TowerDefence.IMC_TowerDefence" "(bIgnoreAllPressedKeysUntilRelease=True,bForceImmediately=False,bNotifyUserSettings=False)")
        (Input|AddMappingContext _returnvalue "/Game/ThreeMatches/Systems/Input/Menu/IMC_Menu.IMC_Menu" 0 "(bIgnoreAllPressedKeysUntilRelease=True,bForceImmediately=False,bNotifyUserSettings=False)")
        (else
          (Input|RemoveMappingContext _returnvalue "/Game/ThreeMatches/Systems/Input/Menu/IMC_Menu.IMC_Menu" "(bIgnoreAllPressedKeysUntilRelease=True,bForceImmediately=False,bNotifyUserSettings=False)")
          (Input|AddMappingContext _returnvalue "/Game/ThreeMatches/Systems/Input/TowerDefence/IMC_TowerDefence.IMC_TowerDefence" 0 "(bIgnoreAllPressedKeysUntilRelease=True,bForceImmediately=False,bNotifyUserSettings=False)"))))))