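; BP_HADCollectibles is a selectable pickup that flies to the castle core and awards Hopes.
; On BeginPlay it sets a rotating-movement pivot from its location and loops a timeline that animates its scale.
; OnSelected fires once, playing a sound and lerping the actor to the core's GrowingMesh.
; On arrival it decrements the owning BP_CollectiblesManager's spawn count, passes HopesToAdd to CallCollected and destroys itself.
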(event EventBeginPlay
  (bind _returnvalue (Transformation|GetActorLocation))
  (bind _returnvalue_2 (Actor|GetActorOfClass "/Game/ThreeMatches/BP_CastleCore.BP_CastleCore_C"))
  (Variables|Default|SetCastleCoreRef _returnvalue_2)
  (bind _result (Math|Float|NegateFloat (.y _returnvalue))
    (:%20%20
      (bind _result_2 (Math|Float|NegateFloat (.x _returnvalue))
        (:%20%20
          (Variables|/Script/Engine.RotatingMovementComponent|SetPivotTranslation (Variables|Default|GetRotatingMovement) (Math|Vector|MakeVector _result_2 _result (.z _returnvalue)))
          (bind _newtrack_0 (Timeline|Timeline Play)
            (:Update
              (Transformation|SetWorldScale3D (Variables|Default|GetDefaultSceneRoot) (Math|Conversions|ToVector(Float) _newtrack_0)))
            (:Finished
              (Timeline|Timeline PlayFromStart))))))))

(event EventOnSelected
  (params (Instigator :type Object%20Object%20Reference) (Hit%20Result :type Hit%20Result%20Structure))
  (bind _castlecoreref (Variables|Default|GetCastleCoreRef))
  (if (not (Variables|Default|GetHasBeenSelected))
    (Variables|Default|SetHasBeenSelected true)
    (Audio|PlaySound2D "/Game/ThreeMatches/Sounds/Cue_HADSelected.Cue_HADSelected" 1.0 1.0 0.0 0 0)
    (Variables|Default|SetStartCollectPoint (Transformation|GetActorLocation))
    (bind _alpha (Timeline|LerpOnDeath PlayFromStart)
      (:Update
        (Utilities|IsValid _castlecoreref
          (:Is%20Valid
            (Transformation|SetActorLocation (Math|Vector|Lerp(Vector) (Variables|Default|GetStartCollectPoint) (Transformation|GetWorldLocation (Variables|/Game/ThreeMatches/Blueprints/BP_GrowingActor.BP_GrowingActor_C|GetGrowingMesh _castlecoreref)) _alpha) false false))))
      (:Finished
        (bind _asbp_collectibles_manager (Utilities|Casting|CastToBP_CollectiblesManager (Components|GetOwner)))
        (bind _result (Math|Integer|DecrementInt (Variables|/Game/ThreeMatches/Blueprints/BP_CollectiblesManager.BP_CollectiblesManager_C|GetCurrentSpawnedCollectibles _asbp_collectibles_manager))
          (:%20%20
            (Variables|/Game/ThreeMatches/Blueprints/BP_CollectiblesManager.BP_CollectiblesManager_C|SetCurrentSpawnedCollectibles _asbp_collectibles_manager _result)
            (Default|CallCollected _asbp_collectibles_manager (Variables|Default|GetHopes%20To%20Add))
            (Actor|DestroyActor)))))))

(fn ConstructionScript)