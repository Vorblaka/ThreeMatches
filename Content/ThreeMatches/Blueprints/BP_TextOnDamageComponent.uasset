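; Damage number component that displays the amount of damage taken as floating text.
; OnDamage resets DamageNumber to its start position, shows it with the amount and sets TextTimeline's play rate.
; Logic to hide the text, offset it sideways by damage parity and turn it toward the player camera exists, but nothing shown here triggers it.
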(event Custom|OnDamage
  (params (DamageAmount :type Integer))
  (bind _damagenumber (Variables|Default|GetDamageNumber))
  (Transformation|SetRelativeLocation _damagenumber (Variables|Default|GetStartTextPosition) false true)
  (Rendering|SetVisibility _damagenumber true false)
  (Rendering|Components|TextRender|SetText _damagenumber (Utilities|Text|ToText(Integer) DamageAmount))
  (Components|Timeline|SetPlayRate (Variables|Default|GetTextTimeline) 1.0))

(event EventBeginPlay)

(event EventTick
  (params (DeltaSeconds :type Float%20%28single-precision%29)))