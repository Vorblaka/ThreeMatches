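; Background actor for the ThreeMatches game that dims the sun light during the match-start cutscene.
; It binds to tower defence player controller events: match start stores the sun's intensity and plays a timeline that scales it down, floored at 5%.
; A skip request resets the timeline time if playback is under nine seconds.
; The start-play FadeIn handler is empty, and a material reveal sequence is left unconnected.
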(event Custom|FadeIn)

(event Custom|MenuPlayPRessed
  (Variables|Default|SetDirectionalLightIntensity (Variables|/Script/Engine.LightComponentBase|GetIntensity (Variables|/Script/Engine.Light|GetLightComponent (Variables|Default|GetSunLight))))
  (bind _railtrack (Timeline|PlayTimeline PlayFromStart)
    (:Update
      (Rendering|Components|Light|SetIntensity (Variables|/Script/Engine.Light|GetLightComponent (Variables|Default|GetSunLight)) (* (Variables|Default|GetDirectionalLightIntensity) (Math|Float|Max(Float) (- 1.0 _railtrack) 0.05))))))

(event Custom|CutsceneSkipped
  (if (< (Components|Timeline|GetPlaybackPosition (Variables|Default|GetPlayTimeline)) 9.0)
    (bind _railtrack (Timeline|PlayTimeline SetNewTime)
      (:Update
        (Rendering|Components|Light|SetIntensity (Variables|/Script/Engine.Light|GetLightComponent (Variables|Default|GetSunLight)) (* (Variables|Default|GetDirectionalLightIntensity) (Math|Float|Max(Float) (- 1.0 _railtrack) 0.05)))))))

(event EventBeginPlay
  (bind _asbp_tower_defence_player_controller (Utilities|Casting|CastToBP_TowerDefencePlayerController (Game|GetPlayerController 0)))
  (EventDispatchers|BindEventtoOnStartPlay _asbp_tower_defence_player_controller (delegate Custom|FadeIn))
  (EventDispatchers|BindEventtoOnMatchStart _asbp_tower_defence_player_controller (delegate Custom|MenuPlayPRessed))
  (EventDispatchers|BindEventtoRequestSkip _asbp_tower_defence_player_controller (delegate Custom|CutsceneSkipped)))

(event Collision|EventActorBeginOverlap
  (params (OtherActor :type Actor%20Object%20Reference)))

(event EventTick
  (params (DeltaSeconds :type Float%20%28single-precision%29)))

(fn ConstructionScript)