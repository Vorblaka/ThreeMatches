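; Actor with an animated growth material on its mesh and pop-up damage numbers.
; AnimateFringe drives GrowthScale and light fringe parameters on a dynamic material through a timeline, then plays a brightness flash.
; OnDamage animates a camera-oriented text component, drifting sideways by damage parity, then hides it.
; SpawnDamageNumber, uncalled here, builds numbers from per-digit Niagara systems with digit textures; SpawnDamageNumberWidget is empty.
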(event Custom|AnimateFringe
  (bind _dynamicmaterialinstance (Variables|Default|GetDynamicMaterialInstance))
  (Components|Timeline|SetPlayRate (Variables|Default|GetLightFringeTimeline) (Variables|Default|GetAnimationSpeed))
  (Components|Timeline|SetPlayRate (Variables|Default|GetFlashTimeline) (Variables|Default|GetFlashSpeed))
  (bind _growthtimeline (Timeline|LightFringeTimeline PlayFromStart)
    (:Update
      (Rendering|Material|SetScalarParameterValue (Variables|Default|GetDynamicMaterialInstance) "GrowthScale" _growthtimeline :!class /Script/Engine.MaterialInstanceDynamic)
      (Rendering|Material|SetScalarParameterValue (Variables|Default|GetDynamicMaterialInstance) "LightFringeSize" (Variables|Default|GetLightFringeSize) :!class /Script/Engine.MaterialInstanceDynamic)
      (Rendering|Material|SetScalarParameterValue (Variables|Default|GetDynamicMaterialInstance) "LightFringeBrightness" (Variables|Default|GetLightFringeBrightness) :!class /Script/Engine.MaterialInstanceDynamic)
      (Rendering|Material|SetVectorParameterValue (Variables|Default|GetDynamicMaterialInstance) "LightFringeColor" (Variables|Default|GetLightFringeColor) :!class /Script/Engine.MaterialInstanceDynamic))
    (:Finished
      (Utilities|FlowControl|Delay 0.05)
      (bind _brightnesstimeline (Timeline|FlashTimeline PlayFromStart)
        (:Update
          (Rendering|Material|SetScalarParameterValue _dynamicmaterialinstance "GrowthScale" 0.99 :!class /Script/Engine.MaterialInstanceDynamic)
          (Rendering|Material|SetScalarParameterValue _dynamicmaterialinstance "LightFringeSize" 1.0 :!class /Script/Engine.MaterialInstanceDynamic)
          (Rendering|Material|SetScalarParameterValue _dynamicmaterialinstance "LightFringeBrightness" (* _brightnesstimeline (Variables|Default|GetFlashBrightness)) :!class /Script/Engine.MaterialInstanceDynamic)
          (Rendering|Material|SetVectorParameterValue _dynamicmaterialinstance "LightFringeColor" (Variables|Default|GetFlashColor) :!class /Script/Engine.MaterialInstanceDynamic))
        (:Finished
          (Utilities|FlowControl|Delay 0.05)
          (Rendering|Material|SetScalarParameterValue (Variables|Default|GetDynamicMaterialInstance) "LightFringeBrightness" 0.0 :!class /Script/Engine.MaterialInstanceDynamic))))))

(event Custom|OnDamage
  (params (DamageAmount :type Integer))
  (bind _returnvalue (Game|GetPlayerCameraManager 0))
  (bind _damagenumber (Variables|Default|GetDamageNumber))
  (bind _returnvalue_2 (Camera|GetCameraRotation _returnvalue))
  (Transformation|SetRelativeLocation _damagenumber (Variables|Default|GetStartTextPosition) false true)
  (Rendering|SetVisibility _damagenumber true false)
  (Rendering|Components|TextRender|SetText _damagenumber (Utilities|Text|ToText(Integer) DamageAmount))
  (Components|Timeline|SetPlayRate (Variables|Default|GetTextTimeline) 1.0)
  (bind _offset (Timeline|TextTimeline PlayFromStart)
    (:Update
      (Transformation|AddLocalOffset _damagenumber (Math|Vector|MakeVector 0.0 (* (.y _offset) (* (- (Math|Integer|%(Integer) DamageAmount 2) 0.5) 2.0)) (.x _offset)) false false)
      (Transformation|SetWorldRotation _damagenumber (Math|Rotator|MakeRotator (+ (.roll _returnvalue_2) 1.8e+02) (+ (.pitch _returnvalue_2) 1.8e+02) (.yaw _returnvalue_2)) false false))
    (:Finished
      (Rendering|SetVisibility _damagenumber false false))))

(event EventBeginPlay
  (bind _returnvalue (Rendering|Material|CreateDynamicMaterialInstance (Variables|Default|GetGrowingMesh) 0 (Rendering|Material|GetMaterial (Variables|Default|GetGrowingMesh) 0) "None" :!class /Script/Engine.PrimitiveComponent))
  (Variables|Default|SetDynamicMaterialInstance _returnvalue)
  (Variables|Default|SetStartTextPosition (Variables|/Script/Engine.SceneComponent|GetRelativeLocation (Variables|Default|GetDamageNumber))))

(fn ConstructionScript)

(fn SpawnDamageNumber
  (params (DamageAmount :type Integer))
  (bind _returnvalue (Transformation|GetActorLocation))
  (for _array_element (Utilities|String|GetCharacterArrayfromString (Utilities|String|ToString(Integer) DamageAmount))
    (bind _returnvalue_2 (Niagara|SpawnSystematLocation "/Game/ThreeMatches/Systems/NS_TextSpawner.NS_TextSpawner" _returnvalue (Math|Rotator|FindLookatRotation _returnvalue (Camera|GetCameraLocation (Game|GetPlayerCameraManager 0)))))
    (bind _output_get (LocalVariables|SetDigitSystem _returnvalue_2))
    (Transformation|AddLocalOffset _output_get (Math|Vector|MakeVector 0.0 (LocalVariables|GetTextOffset) 0.0) false false)
    (LocalVariables|SetTextOffset (+ (LocalVariables|GetTextOffset) 25.0))
    (Niagara|SetTextureObject (LocalVariables|GetDigitSystem) "user.Digit" (Utilities|Select :Index (Math|Conversions|ToInteger(Byte) _array_element) :Option%200 "/Game/KenneyAssets/Numbers/keyboard_0.keyboard_0" :Option%201 "/Game/KenneyAssets/Numbers/keyboard_1.keyboard_1" :Option%202 "/Game/KenneyAssets/Numbers/keyboard_2.keyboard_2" :Option%203 "/Game/KenneyAssets/Numbers/keyboard_3.keyboard_3" :Option%204 "/Game/KenneyAssets/Numbers/keyboard_4.keyboard_4" :Option%205 "/Game/KenneyAssets/Numbers/keyboard_5.keyboard_5" :Option%206 "/Game/KenneyAssets/Numbers/keyboard_6.keyboard_6" :Option%207 "/Game/KenneyAssets/Numbers/keyboard_7.keyboard_7" :Option%208 "/Game/KenneyAssets/Numbers/keyboard_8.keyboard_8" :Option%209 "/Game/KenneyAssets/Numbers/keyboard_9.keyboard_9"))
    (Development|PrintString "Hello")))

(fn SpawnDamageNumberWidget)